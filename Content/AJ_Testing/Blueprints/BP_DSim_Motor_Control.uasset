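; Test Blueprint for linking to a CKAS driving-sim motion platform through SimCorDX over local UDP, using ObjectDeliverer.
; BeginPlay opens the socket, resends an ID message every three seconds and prints any replies.
; Holding A or D ramps a clamped Speed up or down, which Tick maps through timeline curves into a printed SmoothSpeed.
; The motion-data send is unconnected, so SmoothSpeed never reaches the simulator.
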(event Custom|Connected
  (params (ClientSocket :type Object%20Deliverer%20Protocol%20Object%20Reference))
  ;[0.75 0.072 0.3771] Create the delivery manager and events
  (Development|PrintString "Connected! (client)"))

(event Custom|Disconnected
  (params (ClientSocket :type Object%20Deliverer%20Protocol%20Object%20Reference))
  ;[0.75 0.072 0.3771] Create the delivery manager and events
  (Development|PrintString "Disconnected (client)"))

(event Custom|Received%20String
  (params (ReceivedString :type String) (FromObject :type Object%20Deliverer%20Protocol%20Object%20Reference))
  ;[0 0.001974 0.3469] Create Delivery Box
  (Development|PrintString (Utilities|String|Append "SimCorDX says: " ReceivedString) true true "(R=0.982251,G=0.000000,B=0.658375,A=1.000000)"))

(event EventTick
  (params (DeltaSeconds :type Float%20%28single-precision%29))
  (if (> (Variables|Default|GetSpeed) 0.0)
    (bind _newtrack_0 (Timeline|SmoothStep SetNewTime)
      (:Update
        (bind _output_get (Variables|Default|SetSmoothSpeed _newtrack_0))
        (Variables|Default|SetSpeedString (Utilities|String|ToString(Float) _output_get))))
    (else
      (bind _newtrack_0_2 (Timeline|NegSmoothStep SetNewTime)
        (:Update
          (bind _output_get_2 (Variables|Default|SetSmoothSpeed _newtrack_0_2))
          (Variables|Default|SetSpeedString (Utilities|String|ToString(Float) _output_get_2))))))
  (Development|PrintString (Variables|Default|GetSpeedString) true true "(R=0.000000,G=1.000000,B=0.116845,A=1.000000)" (Utilities|Time|GetWorldDeltaSeconds))
  (Development|PrintString (Utilities|String|ToString(Float) (Variables|Default|GetSpeed)) true true "(R=1.000000,G=0.000000,B=0.058415,A=1.000000)" (Utilities|Time|GetWorldDeltaSeconds)))

(event EventBeginPlay
  (bind _returnvalue (Utilities|String|Append "#id " "MotionTest" "\\n"))
  (Input|EnableInput (Game|GetPlayerController 0))
  ;[0.75 0.072 0.3771] Create the delivery manager and events
  (bind _output_get (Variables|ObjectDeliverer|SetObjDelivererMgr (Class|ObjectDelivererManager|CreateObjectDelivererManager true)))
  (EventDispatchers|BindEventtoConnected _output_get (delegate Custom|Connected))
  (EventDispatchers|BindEventtoDisconnected _output_get (delegate Custom|Disconnected))
  ;[0 0.001974 0.3469] Create Delivery Box
  (bind _output_get_2 (Variables|ObjectDeliverer|SetStringDeliveryBox (Class|DeliveryBoxFactory|CreateUtf8StringDeliveryBox)))
  (EventDispatchers|BindEventtoReceived _output_get_2 (delegate Custom|Received%20String))
  ;[0.072 0.75 0.3771] start deliverer
  (Class|ObjectDelivererManager|Start (Variables|ObjectDeliverer|GetObjDelivererMgr) (Class|ProtocolFactory|CreateProtocolUdpSocketSender "127.0.0.1" 1288) (Class|PacketRuleFactory|CreatePacketRuleNodivision) (Variables|ObjectDeliverer|GetStringDeliveryBox)) ; Creates Initial Connect to SimCorDx
  ;[0.75 0.7387 0.072] Sending Initial message
  (Class|Utf8StringDeliveryBox|Send (Variables|ObjectDeliverer|GetStringDeliveryBox) _returnvalue :!label _label) ; Let's make this sent every 3 seconds?
  (Development|PrintString _returnvalue true true "(R=1.000000,G=0.093222,B=0.083274,A=1.000000)")
  (Utilities|FlowControl|Delay 3.0)
  (goto _label))

(event Input|KeyboardEvents|A
  (params (Key :type Key%20Structure :default "None"))
  (:Pressed
    (Variables|Default|SetTurningRight true)
    (if (Variables|Default|GetTurningRight) :!label _label
      (Variables|Default|SetSpeed (+ (Variables|Default|GetSpeed) 0.05))
      (if (> (Variables|Default|GetSpeed) 1.0)
        (Variables|Default|SetSpeed 1.0))
      (Utilities|FlowControl|Delay 0.05)
      (goto _label)))
  (:Released
    (Variables|Default|SetTurningRight false)))

(event Input|KeyboardEvents|D
  (params (Key :type Key%20Structure :default "None"))
  (:Pressed
    (Variables|Default|SetTurningLeft true)
    (if (Variables|Default|GetTurningLeft) :!label _label
      (Variables|Default|SetSpeed (+ (Variables|Default|GetSpeed) -0.05))
      (if (< (Variables|Default|GetSpeed) -1.0)
        (Variables|Default|SetSpeed -1.0))
      (Utilities|FlowControl|Delay 0.05)
      (goto _label)))
  (:Released
    (Variables|Default|SetTurningLeft false)))

(fn ConstructionScript)